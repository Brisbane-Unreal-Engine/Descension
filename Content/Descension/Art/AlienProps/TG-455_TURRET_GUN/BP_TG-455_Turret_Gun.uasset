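; BP_TG-455_Turret_Gun is an alien-prop turret gun actor that can be aimed in yaw and pitch.
; RotateLeft turns the TurretRotator component in yaw, while RotateUp tilts TurretElevator in pitch within clamped limits.
; Both functions take an axis value scaled by frame delta time and a fixed speed.
; The event graph and construction script are empty, so nothing here calls them or handles firing.
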(fn `Rotate Left`
  (params (AxisValue :type "Float (double-precision)"))
  (bind _turretrotator (`self.TurretRotator`))
  (`SceneComponent.K2_SetRelativeRotation` _turretrotator (`KismetMathLibrary.MakeRotator` (.roll (`SceneComponent.RelativeRotation` _turretrotator)) (.pitch (`SceneComponent.RelativeRotation` _turretrotator)) (+ (.yaw (`SceneComponent.RelativeRotation` _turretrotator)) (* (* AxisValue (`GameplayStatics.GetWorldDeltaSeconds`)) 20.0))) false false))

(fn `Rotate Up`
  (params (AxisValue :type "Float (double-precision)"))
  (bind _turretelevator (`self.TurretElevator`))
  (`SceneComponent.K2_SetRelativeRotation` _turretelevator (`KismetMathLibrary.MakeRotator` (.roll (`SceneComponent.RelativeRotation` _turretelevator)) (`KismetMathLibrary.FClamp` (+ (.pitch (`SceneComponent.RelativeRotation` _turretelevator)) (* (* AxisValue (`GameplayStatics.GetWorldDeltaSeconds`)) 10.0)) -10.0 25.0) (.yaw (`SceneComponent.RelativeRotation` _turretelevator))) false false))

(fn `UserConstructionScript`)